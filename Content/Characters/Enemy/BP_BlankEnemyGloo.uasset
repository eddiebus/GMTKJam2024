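; Enemy character Blueprint that shows a floating health display through a WBP_Enemy widget.
; On BeginPlay it caches the widget, then each tick pushes Health and MaxHealth to it.
; UpdateWidgetPosition also runs every tick, placing the widget above the enemy at an offset scaled by the Sphere component's radius.
; CheckVisionToPlayer is an empty stub with an unconnected actor search.
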(event `self.ReceiveBeginPlay`
  (`parent.ReceiveBeginPlay`)
  (bind _aswbp_enemy (cast `/Game/AI/Enemy_UI/WBP_Enemy` (`WidgetComponent.GetWidget` (`self.Widget`))))
  (set `self.DisplayWidget` _aswbp_enemy))

(event `self.ReceiveTick`
  (params (DeltaSeconds :type "Float (single-precision)"))
  (`parent.ReceiveTick` DeltaSeconds)
  (`self.UpdateWidgetPosition`)
  (`/Game/AI/Enemy_UI/WBP_Enemy.Set Display Health` (`self.DisplayWidget`) (`self.Health`) (`self.MaxHealth`)))

(fn `CheckVisionToPlayer`)

(fn `UpdateWidgetPosition`
  (`SceneComponent.K2_SetWorldLocation` (`self.Widget`) (+ (`self.Get World Position`) (* (`KismetMathLibrary.Vector_Up`) (`.SphereRadius` (`KismetSystemLibrary.GetComponentBounds` (`self.Sphere`))) 1.5)) false false))

(fn `UserConstructionScript`
  (`parent.UserConstructionScript`))