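; BP_Glooball is a physics-driven ball combatant that rolls and jumps by impulses, collecting weapons on overlap.
; Hits push other Glooballs and deal base, weapon and level damage, scaled by the victim's speed; kills grant XP toward levels.
; Tick caps horizontal speed, sizes the ball by health and level, sets mass from XP, draws debug shapes and respawns strays.
; Navigation path and nearest-Gloo helpers are also provided.
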(event `self.ReceiveBeginPlay`
  (set `self.InitLocation` (`self.Get World Position`))
  (bind _asplayer_controller (cast `PlayerController` (`self.GetController`)))
  (`EnhancedInputSubsystemInterface.AddMappingContext` (pcsubsystem `EnhancedInputLocalPlayerSubsystem` _asplayer_controller) "/Game/Other/Input/IMC_InputMap.IMC_InputMap" 0 (struct)))

(event `self.ReceiveTick`
  (params (DeltaSeconds :type "Float (single-precision)"))
  (`self.Clamp Velocity`)
  (`self. Draw Debug`)
  (`self.UpdateGlooSize`)
  (`self.UpdateGlooMass`)
  (if (> (`KismetMathLibrary.VSize` (`self.Get World Position`)) 10000.0)
    (`self.Set World Position` (`self.InitLocation`))
    (`self.SetVelocity` (0.0 0.0 0.0))))

(event `self.ReceiveActorBeginOverlap`
  (params (OtherActor :type "Actor Object Reference"))
  (bind _asbp_gloo_weapon (cast `/Game/Actors/BP_GlooWeapon` OtherActor))
  (`/Game/Actors/BP_GlooWeapon.AttachToGloo` _asbp_gloo_weapon self)
  (`BlueprintSetLibrary.Set_Add` (`self.Weapons`) _asbp_gloo_weapon))

(event `self.ReceiveHit`
  (params (MyComp :type "PrimitiveComponent Object Reference") (Other :type "Actor Object Reference") (OtherComp :type "PrimitiveComponent Object Reference") (bSelfMoved :type Boolean) (HitLocation :type "Vector Structure") (HitNormal :type "Vector Structure") (NormalImpulse :type "Vector Structure") (Hit :type "HitResult Structure (by ref)"))
  (`self.Attack Gloo` MyComp Other))

(fn ` Draw Debug`
  (bind _rootsphere (`self.RootSphere`))
  (bind _rootsphere_2 (`self.RootSphere`))
  (bind _returnvalue (`SceneComponent.K2_GetComponentLocation` _rootsphere))
  (bind _returnvalue_2 (`SceneComponent.K2_GetComponentLocation` (`self.RootSphere`)))
  (`KismetSystemLibrary.DrawDebugLine` _returnvalue (+ _returnvalue (* (`KismetMathLibrary.Normal` (`SceneComponent.GetComponentVelocity` _rootsphere)) (* (`.SphereRadius` (`KismetSystemLibrary.GetComponentBounds` _rootsphere)) 4.0))) (struct) 0.0 3.0)
  (`KismetSystemLibrary.DrawDebugLine` _returnvalue_2 (+ _returnvalue_2 (* (`self.GetFloorNormal`) (* (`.SphereRadius` (`KismetSystemLibrary.GetComponentBounds` (`self.RootSphere`))) 2.2))) (struct :`R` 0.199314 :`G` 1.0 :`A` 1.0) 0.0 3.0)
  (`KismetSystemLibrary.DrawDebugSphere` (`SceneComponent.K2_GetComponentLocation` _rootsphere_2) (* (`.SphereRadius` (`KismetSystemLibrary.GetComponentBounds` _rootsphere_2)) 2.0) 12 (struct :`R` 0.4814 :`B` 1.0 :`A` 1.0))
  (return))

(fn `AddExp`
  (params (Exp :type "Float (double-precision)"))
  (set `self.Exp` (+ (`self.Exp`) Exp))
  (if (> (`self.Exp`) (`self.Get Exp Goal`))
    (`/Engine/EditorBlueprintResources/StandardMacros.IncrementInt` (`self.Level`)
      (:`  `
        (set `self.Exp` 0.0)
        (set `self.MaxHealth` (+ 0.0 50.0))
        (return)))
    (else
      (return))))

(fn `AddHealth`
  (params (HP :type "Float (double-precision)"))
  (set `self.Health` (+ HP (`self.Health`))))

(fn `ApplyDamage`
  (params (Value :type "Float (double-precision)"))
  (returns (KillingBlow :type Boolean))
  (locals (WasAlive :type Boolean))
  (if (not (`self.Invincible`))
    (set `self.Health` (- (`self.Health`) (* Value (/ (`self.GetCurrentVelocity`) 100.0))))
    (`self.OnDamageTaken`)
    (if (<= (`self.Health`) 0.0)
      (`self.OnDeath`)
      (`self.Defeat`)
      (return true)
      (else
        (return false)))
    (else
      (return false))))

(fn `AttachWeapon`
  (params (Weapon :type "/Game/Actors/BP_GlooWeapon Object Reference"))
  (`/Game/Actors/BP_GlooWeapon.AttachToGloo` Weapon self)
  (`BlueprintSetLibrary.Set_Add` (`self.Weapons`) Weapon))

(fn `Attack Gloo`
  (params (A :type "Object Object Reference") (InputPin :type "Actor Object Reference"))
  (locals (OtherXP :type "Float (double-precision)"))
  (bind _position (`self.Get World Position`))
  (if (== A (`self.RootSphere`))
    (bind _asbp_glooball (cast `/Game/Characters/Player/BP_Glooball` InputPin))
    (set `local.OtherXP` (`/Game/Characters/Player/BP_Glooball.ExpDrop` _asbp_glooball))
    (`self.Push Gloo` _asbp_glooball (`KismetMathLibrary.ClampVectorSize` (- (`self.Get World Position` _asbp_glooball) (`self.Get World Position`)) 0.0 3.0))
    (bind _killingblow (`self.ApplyDamage` _asbp_glooball (`self.GetDamageValue`)))
    (if _killingblow
      (`self.AddExp` (`local.OtherXP`))
      (else
        ;[1 1 1] PlaySound'
        (if (`self.HasWeapon`)
          (`GameplayStatics.PlaySoundAtLocation` "/Game/Sound/SFX/Sword/SC_SwordClash.SC_SwordClash" _position (struct) (`/Game/Other/OptionSaveGame.GetSFXVol` (`/Game/Other/GameInstance/GlooInstanceHelper.GetGameOptions`)) 1.0 0.0 null null null null)
          (else
            (`GameplayStatics.PlaySoundAtLocation` "/Game/Sound/SFX/Punch/SC_Punch.SC_Punch" _position (struct) 0.4 1.0 0.0 null null null null)))))))

(fn `CalcGlooSize`
  (returns (Size :type "Float (double-precision)"))
  (return (+ (`KismetMathLibrary.FClamp` (+ (`self.GetHealthPercentage`) 0.3)) (* (`KismetMathLibrary.Conv_IntToDouble` (`self.Level`)) 0.1))))

(fn `Clamp Velocity`
  (locals (VelocityArray :type "Array of Float (double-precision)") (ArrayIndex :type Integer) (ReadElement :type "Float (double-precision)") (`Speed Diff` :type "Float (double-precision)"))
  (bind _returnvalue (`SceneComponent.GetComponentVelocity` (`self.RootSphere`)))
  (`PrimitiveComponent.SetPhysicsLinearVelocity` (`self.RootSphere`) (`KismetMathLibrary.MakeVector` (.x (`KismetMathLibrary.ClampVectorSize` _returnvalue 0.0 (`self.MaxSpeed`))) (.y (`KismetMathLibrary.ClampVectorSize` _returnvalue 0.0 (`self.MaxSpeed`))) (.z _returnvalue)) false "None"))

(fn `Defeat`
  (`self.OnDeath`)
  (`self.K2_DestroyActor`))

(fn `Get Exp Goal`
  (returns (TargetExp :type "Float (double-precision)"))
  (return (* (`KismetMathLibrary.Conv_IntToDouble` (`self.Level`)) 40.0 (`self.TargetXPMultiplier`))))

(fn `Get EXPPercental`
  (returns (Percental :type "Float (double-precision)"))
  (return (/ (`self.Exp`) (`self.Get Exp Goal`))))

(fn `Get Nearest Gloo`
  (params (GlooToCheck :type "Array of /Game/Characters/Player/BP_Glooball Object Reference"))
  (returns (Nearest :type "/Game/Characters/Player/BP_Glooball Object Reference"))
  (locals (CurrentGloo :type "/Game/Characters/Player/BP_Glooball Object Reference") (NearestGloo :type "/Game/Characters/Player/BP_Glooball Object Reference") (Distance :type "Float (double-precision)"))
  (set `local.Distance` 1000000000000.0)
  (for _array_element GlooToCheck
    (bind _output_get (set `local.CurrentGloo` _array_element))
    (if (< (`KismetMathLibrary.Abs` (`KismetMathLibrary.VSize` (- (`self.Get World Position`) (`self.Get World Position` _output_get)))) (`local.Distance`))
      (set `local.NearestGloo` (`local.CurrentGloo`))))
  (return (`local.NearestGloo`)))

(fn `Get Random Nav Path`
  (returns (ResultPath :type "NavigationPath Object Reference"))
  (bind _position (`self.Get World Position`))
  (bind _returnvalue (`NavigationSystemV1.FindPathToLocationSynchronously` _position (`NavigationSystemV1.K2_GetRandomReachablePointInRadius` _position 100000000.0 null null) null null))
  (return _returnvalue))

(fn `Get World Position`
  (returns (Position :type "Vector Structure"))
  (if (`KismetSystemLibrary.IsValid` (`self.RootSphere`))
    (return (`SceneComponent.K2_GetComponentLocation` (`self.RootSphere`)))
    (else
      (return (0.0 0.0 0.0)))))

(fn `GetCurrentVelocity`
  (returns (Speed :type "Float (double-precision)"))
  (return (`KismetMathLibrary.Abs` (`KismetMathLibrary.VSize` (`SceneComponent.GetComponentVelocity` (`self.RootSphere`))))))

(fn `GetDamageValue`
  (returns (TrueDamageValue :type "Float (double-precision)"))
  (locals (DamageTotal :type "Float (double-precision)"))
  (set `local.DamageTotal` 0.0)
  (bind _result (`BlueprintSetLibrary.Set_ToArray` (`self.Weapons`)))
  (for _array_element _result
    (set `local.DamageTotal` (+ (`local.DamageTotal`) (`/Game/Actors/BP_GlooWeapon.DamagePoints` _array_element))))
  (return (+ (`local.DamageTotal`) (`self.BaseDamage`) (* (`KismetMathLibrary.Conv_IntToDouble` (`self.Level`)) 1.2))))

(fn `GetFloorNormal`
  (returns (FloorNormal :type "Vector Structure") (OnFloor :type Boolean))
  (locals (ResultHit :type "HitResult Structure") (DidHit :type Boolean))
  (bind _rootsphere (`self.RootSphere`))
  (bind _returnvalue (`SceneComponent.K2_GetComponentLocation` _rootsphere))
  (bind (_outhit _returnvalue_2) (`KismetSystemLibrary.LineTraceSingleForObjects` _returnvalue (+ _returnvalue (* (* (`.SphereRadius` (`KismetSystemLibrary.GetComponentBounds` _rootsphere)) 2.0) (`KismetMathLibrary.Vector_Down`))) (`|MakeArray` "ObjectTypeQuery1" :!type "EObjectTypeQuery Enum")))
  (bind _output_get (set `local.DidHit` _returnvalue_2))
  (set `local.ResultHit` _outhit)
  (if _output_get
    (return (`.Normal` (`GameplayStatics.BreakHitResult` (`local.ResultHit`))) (`local.DidHit`))
    (else
      (return (`KismetMathLibrary.Vector_Up`) (`local.DidHit`)))))

(fn `GetHealthPercentage`
  (returns (Percent :type "Float (double-precision)"))
  (return (/ (`self.Health`) (`self.MaxHealth`))))

(fn `GetMovementSpeed`
  (returns (Speed :type "Float (double-precision)"))
  (return (* (`PrimitiveComponent.GetMass` (`self.RootSphere`)) 2.0 (`self.RollSpeed`))))

(fn `GetPathToPoint`
  (params (TargetPoint :type "Vector Structure") (Radius :type "Float (double-precision)" :default 100.0))
  (returns (NewParam :type "NavigationPath Object Reference"))
  (bind _returnvalue (`NavigationSystemV1.FindPathToLocationSynchronously` (`self.Get World Position`) TargetPoint null null))
  (return _returnvalue))

(fn `GetRootComponent`
  (returns (NewParam :type "SceneComponent Object Reference"))
  (return (`self.RootSphere`)))

(fn `HasWeapon`
  (returns (Bool :type Boolean))
  (return (> (`BlueprintSetLibrary.Set_Length` (`self.Weapons`)) 0)))

(fn `HealPercental`
  (params (Percental :type "Float (double-precision)"))
  (set `self.Health` (+ (`self.Health`) (* Percental (`self.MaxHealth`)))))

(fn `Jump`
  (bind (_floornormal _onfloor) (`self.GetFloorNormal`))
  (if _onfloor
    (`PrimitiveComponent.AddImpulse` (`self.RootSphere`) (* (* (* _floornormal (`self.JumpStrength`)) (`PrimitiveComponent.GetMass` (`self.RootSphere`))) 10.0) "None" true)
    (else
      (return))))

(fn `Push Gloo`
  (params (Force :type "Vector Structure"))
  (`PrimitiveComponent.AddImpulse` (`self.RootSphere`) (* Force (* 1.0 1.7 (* (`KismetMathLibrary.RandomFloat`) 100.0))) "None" true))

(fn `Roll`
  (params (Direction :type "Vector2D Structure"))
  (bind (_x _y) (`KismetMathLibrary.BreakVector2D` Direction))
  (`PrimitiveComponent.AddImpulse` (`self.RootSphere`) (* (`KismetMathLibrary.MakeVector` _x _y) (`self.GetMovementSpeed`)) "None" true))

(fn `Set World Position`
  (params (NewLocation :type "Vector Structure"))
  (`SceneComponent.K2_SetRelativeLocation` (`self.RootSphere`) NewLocation false true))

(fn `SetVelocity`
  (params (NewVelocity :type "Vector Structure"))
  (`PrimitiveComponent.SetPhysicsLinearVelocity` (`self.RootSphere`) NewVelocity false "None"))

(fn `ToggleInvincible`
  (params (NewInvincible :type Boolean))
  (set `self.Invincible` NewInvincible))

(fn `UpdateGlooMass`
  (`PrimitiveComponent.SetMassOverrideInKg` (`self.RootSphere`) "None" (* 30.0 (`KismetMathLibrary.FClamp` (/ (`self.Exp`) 100.0) 1.0 100000.0)) true))

(fn `UpdateGlooSize`
  (locals (ScaleVector :type "Vector Structure"))
  (set `local.ScaleVector` (`KismetMathLibrary.Vector_One`))
  (set `local.ScaleVector` (* (`local.ScaleVector`) (`KismetMathLibrary.FClamp` (+ (`self.GetHealthPercentage`) 0.3))))
  (`SceneComponent.K2_SetRelativeTransform` (`self.RootSphere`) (`KismetMathLibrary.MakeTransform` (.location (`SceneComponent.GetRelativeTransform` (`self.RootSphere`))) (.rotation (`SceneComponent.GetRelativeTransform` (`self.RootSphere`))) (* (`KismetMathLibrary.Vector_One`) (`self.CalcGlooSize`))) false false))

(fn `UserConstructionScript`
  (set `self.MaxHealth` (`self.Health`)))