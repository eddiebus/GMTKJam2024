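; Player-controlled rolling ball pawn that adds the Enhanced Input mapping and turns input into rolling, jumping, camera look and pausing.
; Movement goes through ProjectToCameraDIrection, whose nodes shown here are all unconnected, into Roll.
; Each tick moves the spring arm above the ball, scaled by CalcGlooSize, clamps look pitch and debug-prints health.
; Defeat clears the mesh, stops physics and calls OnDeath; pause opens WB_PauseMenu.
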(event `self.ReceiveBeginPlay`
  ;[1 1 1] Set Player Input
  (`parent.ReceiveBeginPlay`)
  (bind _asplayer_controller (cast `PlayerController` (`self.GetController`)))
  (`EnhancedInputSubsystemInterface.AddMappingContext` (pcsubsystem `EnhancedInputLocalPlayerSubsystem` _asplayer_controller) "/Game/Other/Input/IMC_InputMap.IMC_InputMap" 0 (struct))
  (set `self.TestPath` (`self.Get Random Nav Path`)))

(event `self.ReceiveTick`
  (params (DeltaSeconds :type "Float (single-precision)"))
  (`parent.ReceiveTick` DeltaSeconds)
  (`self.Update Cam Location`)
  (`KismetSystemLibrary.PrintString` (`KismetStringLibrary.Conv_DoubleToString` (`self.GetHealthPercentage`))))

(event `EnhancedInput|/Game/ThirdPerson/Input/Actions/IA_Move`
  (params (ActionValue :type "Vector2D Structure") (ElapsedSeconds :type "Float (double-precision)") (TriggeredSeconds :type "Float (double-precision)") (InputAction :type "InputAction Object Reference" :default "/Game/ThirdPerson/Input/Actions/IA_Move.IA_Move"))
  (bind (_x _y) (`KismetMathLibrary.BreakVector2D` ActionValue))
  (bind _camera (`self.Camera`))
  (:`Triggered`
    (`self.Roll` (`KismetMathLibrary.Conv_VectorToVector2D` (`KismetMathLibrary.ClampVectorSize` (+ (* (`SceneComponent.GetRightVector` _camera) _x) (* (`SceneComponent.GetForwardVector` _camera) _y)) 0.0 1.0)))))

(event `EnhancedInput|/Game/ThirdPerson/Input/Actions/IA_Jump`
  (params (ActionValue :type Boolean) (ElapsedSeconds :type "Float (double-precision)") (TriggeredSeconds :type "Float (double-precision)") (InputAction :type "InputAction Object Reference" :default "/Game/ThirdPerson/Input/Actions/IA_Jump.IA_Jump"))
  (:`Triggered`
    (`self.Jump`)))

(event `EnhancedInput|/Game/ThirdPerson/Input/Actions/IA_Look`
  (params (ActionValue :type "Vector2D Structure") (ElapsedSeconds :type "Float (double-precision)") (TriggeredSeconds :type "Float (double-precision)") (InputAction :type "InputAction Object Reference" :default "/Game/ThirdPerson/Input/Actions/IA_Look.IA_Look"))
  ;[1 1 1] Update Camera Look
  (:`Triggered`
    (set `self.LookVector` (+ (`self.LookVector`) ActionValue))
    (`SceneComponent.K2_SetRelativeRotation` (`self.SpringArm`) (`KismetMathLibrary.MakeRotator` 0.0 (* (.y (`self.LookVector`)) -1.0) (.x (`self.LookVector`))) false false)))

(event `EnhancedInput|/Game/Other/Input/IA_Pause`
  (params (ActionValue :type Boolean) (ElapsedSeconds :type "Float (double-precision)") (TriggeredSeconds :type "Float (double-precision)") (InputAction :type "InputAction Object Reference" :default "/Game/Other/Input/IA_Pause.IA_Pause"))
  (bind _returnvalue (`GameplayStatics.GetPlayerController` 0))
  (:`Triggered`
    (`GameplayStatics.SetGamePaused` true)
    (bind _returnvalue_2 (`|CreateWidget` "/Game/UI/WB_PauseMenu.WB_PauseMenu_C" _returnvalue))
    (`UserWidget.AddToViewport` _returnvalue_2 0)
    (`WidgetBlueprintLibrary.SetInputMode_UIOnlyEx` _returnvalue _returnvalue_2)
    (set `PlayerController.bShowMouseCursor` true _returnvalue)))

(fn `ClampLookDirection`
  (params (MaxVertAngle :type "Float (double-precision)" :default 75.0))
  (bind _returnvalue (`|Copy` MaxVertAngle))
  (if (> (.y (`self.LookVector`)) (`KismetSystemLibrary.MakeLiteralDouble` MaxVertAngle))
    (set `self.LookVector` (`KismetMathLibrary.MakeVector` (.x (`self.LookVector`)) _returnvalue))
    (else
      (bind _result (`/Engine/EditorBlueprintResources/StandardMacros.NegateFloat` _returnvalue)
        (:`  `
          (if (< (.y (`self.LookVector`)) _result)
            (set `self.LookVector` (`KismetMathLibrary.MakeVector` (.x (`self.LookVector`)) _result))))))))

(fn `Defeat`
  (bind _ballmesh (`self.BallMesh`))
  (`StaticMeshComponent.SetStaticMesh` _ballmesh null)
  (`PrimitiveComponent.SetSimulatePhysics` _ballmesh false)
  (`PrimitiveComponent.SetSimulatePhysics` (`self.RootSphere`) false)
  (`self.OnDeath`)
  (return))

(fn `Update Cam Location`
  (`SceneComponent.K2_SetWorldLocation` (`self.SpringArm`) (+ (`self.Get World Position`) (* (`KismetMathLibrary.Vector_Up`) (`self.CalcGlooSize`) 100.0)) false false)
  (`self.ClampLookDirection` 75.0))

(fn `UserConstructionScript`
  (`parent.UserConstructionScript`))