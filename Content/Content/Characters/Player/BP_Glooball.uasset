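; BP_Glooball is the player's physics-driven ball, which rolls and jumps by impulses applied to its Sphere.
; BeginPlay adds the input mapping context, while Roll and Jump expose movement without being called in this graph.
; A downward line trace scaled to the ball's bounds supplies the floor normal, gating Jump and setting its direction.
; Tick clamps X and Y velocity separately to MaxSpeed, leaving Z free, and draws movement and floor debug info.
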(event `self.ReceiveBeginPlay`
  (bind _asplayer_controller (cast `PlayerController` (`self.GetController`)))
  (`EnhancedInputSubsystemInterface.AddMappingContext` (pcsubsystem `EnhancedInputLocalPlayerSubsystem` _asplayer_controller) "/Game/Content/Other/Input/IMC_InputMap.IMC_InputMap" 0 (struct)))

(event `self.ReceiveTick`
  (params (DeltaSeconds :type "Float (single-precision)"))
  (`self.Clamp Velocity`)
  (`KismetSystemLibrary.PrintString` (`KismetStringLibrary.Concat_StrStr` "Normal " (`KismetStringLibrary.Conv_VectorToString` (`self.GetFloorNormal`)) "| Velocity : " (`KismetStringLibrary.Conv_VectorToString` (`SceneComponent.GetComponentVelocity` (`self.Sphere`)))))
  (`self. Draw Debug`))

(fn ` Draw Debug`
  (bind _sphere (`self.Sphere`))
  (bind _sphere_2 (`self.Sphere`))
  (bind _returnvalue (`SceneComponent.K2_GetComponentLocation` _sphere))
  (bind _returnvalue_2 (`SceneComponent.K2_GetComponentLocation` (`self.Sphere`)))
  (`KismetSystemLibrary.DrawDebugLine` _returnvalue (+ _returnvalue (* (`KismetMathLibrary.Normal` (`SceneComponent.GetComponentVelocity` _sphere)) (* (`.SphereRadius` (`KismetSystemLibrary.GetComponentBounds` _sphere)) 10.0))))
  (`KismetSystemLibrary.DrawDebugLine` _returnvalue_2 (+ _returnvalue_2 (* (`self.GetFloorNormal`) (* (`.SphereRadius` (`KismetSystemLibrary.GetComponentBounds` (`self.Sphere`))) 5.0))) (struct :`R` 0.199314 :`G` 1.0 :`A` 1.0) 0.0 3.0)
  (`KismetSystemLibrary.DrawDebugSphere` (`SceneComponent.K2_GetComponentLocation` _sphere_2) (* (`.SphereRadius` (`KismetSystemLibrary.GetComponentBounds` _sphere_2)) 2.0) 12 (struct :`R` 0.4814 :`B` 1.0 :`A` 1.0))
  (return))

(fn `Clamp Velocity`
  (locals (VelocityArray :type "Array of Float (double-precision)") (ArrayIndex :type Integer) (ReadElement :type "Float (double-precision)") (`Speed Diff` :type "Float (double-precision)"))
  (bind _arrayindex (`local.ArrayIndex`))
  (bind _velocityarray (`local.VelocityArray`))
  (bind _velocityarray_2 (`local.VelocityArray`))
  (bind _output_get (set `local.VelocityArray` (`|MakeArray` (.x (`SceneComponent.GetComponentVelocity` (`self.Sphere`))) (.y (`SceneComponent.GetComponentVelocity` (`self.Sphere`))) (.z (`SceneComponent.GetComponentVelocity` (`self.Sphere`))))))
  (for (_array_element _array_index) _output_get
    (set `local.ReadElement` _array_element)
    (set `local.ArrayIndex` _array_index)
    (if (!= (`local.ArrayIndex`) 2)
      (if (> (`KismetMathLibrary.Abs` (`local.ReadElement`)) (`self.MaxSpeed`))
        (if (> (`local.ReadElement`) 0.0)
          (`KismetArrayLibrary.Array_Set` _velocityarray _arrayindex (`self.MaxSpeed`))
          (else
            (bind _result (`/Engine/EditorBlueprintResources/StandardMacros.NegateFloat` (`|Copy` (`self.MaxSpeed`)))
              (:`  `
                (`KismetArrayLibrary.Array_Set` _velocityarray _arrayindex _result))))))))
  (`PrimitiveComponent.SetPhysicsLinearVelocity` (`self.Sphere`) (`KismetMathLibrary.MakeVector` (`|GetArrayItem` _velocityarray_2) (`|GetArrayItem` _velocityarray_2 1) (`|GetArrayItem` _velocityarray_2 2)) false "None"))

(fn `Get World Position`
  (returns (Position :type "Vector Structure"))
  (return (`SceneComponent.K2_GetComponentLocation` (`self.Sphere`))))

(fn `GetFloorNormal`
  (returns (FloorNormal :type "Vector Structure") (OnFloor :type Boolean))
  (locals (ResultHit :type "HitResult Structure") (DidHit :type Boolean))
  (bind _sphere (`self.Sphere`))
  (bind _returnvalue (`SceneComponent.K2_GetComponentLocation` _sphere))
  (bind (_outhit _returnvalue_2) (`KismetSystemLibrary.LineTraceSingleForObjects` _returnvalue (+ _returnvalue (* (* (`.SphereRadius` (`KismetSystemLibrary.GetComponentBounds` _sphere)) 2.0) (`KismetMathLibrary.Vector_Down`))) (`|MakeArray` "ObjectTypeQuery1" :!type "EObjectTypeQuery Enum")))
  (bind _output_get (set `local.DidHit` _returnvalue_2))
  (set `local.ResultHit` _outhit)
  (if _output_get
    (return (`.Normal` (`GameplayStatics.BreakHitResult` (`local.ResultHit`))) (`local.DidHit`))
    (else
      (return (`KismetMathLibrary.Vector_Up`) (`local.DidHit`)))))

(fn `Jump`
  (bind (_floornormal _onfloor) (`self.GetFloorNormal`))
  (if _onfloor
    (`PrimitiveComponent.AddImpulse` (`self.Sphere`) (* (* (* _floornormal (`self.JumpStrength`)) (`PrimitiveComponent.GetMass` (`self.Sphere`))) 5.0) "None" true)
    (else
      (return))))

(fn `Roll`
  (params (Direction :type "Vector2D Structure"))
  (bind (_x _y) (`KismetMathLibrary.BreakVector2D` Direction))
  (`PrimitiveComponent.AddImpulse` (`self.Sphere`) (* (`KismetMathLibrary.MakeVector` _x _y) (* (`PrimitiveComponent.GetMass` (`self.Sphere`)) 0.5)) "None" true)
  (if (> (`KismetMathLibrary.VSize` (`SceneComponent.GetComponentVelocity` (`self.Sphere`))) (`self.MaxSpeed`))
    _))

(fn `UserConstructionScript`)