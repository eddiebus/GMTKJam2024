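; BP_GlooWeapon is a weapon actor that sticks to a BP_Glooball when it overlaps one.
; AttachToGloo attaches it once to the ball's root, keeping world location but snapping rotation and scale, then disables mesh collision and physics through TogglePhysics.
; It then clamps the mesh's relative offset to 80% of the ball's bounds extent length, keeping the weapon close to the ball.
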(event `self.ReceiveActorBeginOverlap`
  (params (OtherActor :type "Actor Object Reference"))
  (bind _asbp_glooball (cast `/Game/Characters/Player/BP_Glooball` OtherActor))
  (`self.AttachToGloo` _asbp_glooball))

(fn `AttachToGloo`
  (params (TargetGloo :type "/Game/Characters/Player/BP_Glooball Object Reference"))
  (locals (TargetBall :type "/Game/Characters/Player/BP_Glooball Object Reference"))
  (bind _output_get (set `local.TargetBall` TargetGloo))
  (if (not (`self.Parented`))
    (bind _returnvalue (`self.K2_AttachToComponent` (`/Game/Characters/Player/BP_Glooball.GetRootComponent` _output_get) "None" "KeepWorld" "SnapToTarget" "SnapToTarget"))
    (if _returnvalue
      (`self.Toggle Physics` false)
      (set `self.Parented` true)
      (`SceneComponent.K2_SetRelativeTransform` (`self.StaticMesh`) (`KismetMathLibrary.MakeTransform` (`KismetMathLibrary.ClampVectorSize` (.location (`SceneComponent.GetRelativeTransform` (`self.StaticMesh`))) 0.0 (* (`KismetMathLibrary.VSize` (`.BoxExtent` (`self.GetActorBounds` (`local.TargetBall`) true false))) 0.8)) (.rotation (`SceneComponent.GetRelativeTransform` (`self.StaticMesh`))) (.scale (`SceneComponent.GetRelativeTransform` (`self.StaticMesh`)))) false false)
      (else
        (return)))
    (else
      (return))))

(fn `Toggle Physics`
  (params (On :type Boolean))
  (bind _staticmesh (`self.StaticMesh`))
  (bind _staticmesh_2 (`self.StaticMesh`))
  (if On
    (`PrimitiveComponent.SetCollisionEnabled` _staticmesh_2 "QueryAndPhysics")
    (`PrimitiveComponent.SetSimulatePhysics` _staticmesh_2 true)
    (else
      (`PrimitiveComponent.SetCollisionEnabled` _staticmesh "NoCollision")
      (`PrimitiveComponent.SetSimulatePhysics` _staticmesh false))))

(fn `UserConstructionScript`)