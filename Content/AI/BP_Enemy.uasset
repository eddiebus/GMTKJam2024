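; BP_Enemy is an AI enemy that chases the player and takes damage when a BP_PlayerBall overlaps its sphere.
; A self-repeating event re-targets the player pawn's "Player"-tagged component every two seconds through AI MoveToLocation.
; Overlap applies damage to the enemy itself, which is scaled up before reducing health.
; Each surviving hit updates the WBP_Enemy health widget and shrinks the actor to a third, while depleted health destroys it.
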(event `self.ReceiveBeginPlay`
  ;[1 1 1] Chase and UI logic
  (`self.ChasePlayer`)
  (bind _aswbp_enemy (cast `/Game/AI/Enemy_UI/WBP_Enemy` (`WidgetComponent.GetUserWidgetObject` (`self.Widget`))))
  (bind _output_get (set `self.WBP Enemy` _aswbp_enemy))
  (set `/Game/AI/Enemy_UI/WBP_Enemy.CurrentHealth` (`self.CurrentHealth`) _output_get)
  (set `/Game/AI/Enemy_UI/WBP_Enemy.MaxHealth` (`self.MaxHealth`) _output_get))

(event `ChasePlayer`
  ;[1 1 1] Chase and UI logic
  (bind _asscene_component (cast `SceneComponent` (`|GetArrayItem` (`self.GetComponentsByTag` (`GameplayStatics.GetPlayerPawn` 0) "/Script/Engine.ActorComponent" "Player"))))
  (`AIController.MoveToLocation` (`AIBlueprintHelperLibrary.GetAIController` self) (`SceneComponent.K2_GetComponentLocation` _asscene_component) -1.0 true true false true null true)
  (`KismetSystemLibrary.Delay` 2.0)
  (`self.ChasePlayer`))

(event `self.Sphere.OnComponentBeginOverlap`
  (params (OverlappedComponent :type "PrimitiveComponent Object Reference") (OtherActor :type "Actor Object Reference") (OtherComp :type "PrimitiveComponent Object Reference") (OtherBodyIndex :type Integer) (bFromSweep :type Boolean) (SweepResult :type "HitResult Structure (by ref)"))
  ;[1 1 1] When the enemy does get damaged
  (cast `/Game/Characters/Player/BP_PlayerBall` OtherActor)
  (`GameplayStatics.ApplyDamage` self 1.0)
  (`KismetSystemLibrary.PrintText` "SOUND"))

(event `self.ReceiveAnyDamage`
  (params (Damage :type "Float (single-precision)") (DamageType :type "DamageType Object Reference") (InstigatedBy :type "Controller Object Reference") (DamageCauser :type "Actor Object Reference"))
  ;[1 1 1] When the enemy gets damaged
  (bind _output_get (set `self.CurrentHealth` (- (`self.CurrentHealth`) (* Damage 100.0))))
  (if (<= (`self.CurrentHealth`) (`self.MinHealth`))
    (`self.K2_DestroyActor`)
    (else
      (`/Game/AI/Enemy_UI/WBP_Enemy.Update Health` (`self.WBP Enemy`) (`KismetMathLibrary.Clamp` _output_get 0 (`self.MaxHealth`)))
      (`self.SetActorScale3D` (* (`self.GetActorScale3D`) (0.33 0.33 0.33))))))

(fn `UserConstructionScript`)