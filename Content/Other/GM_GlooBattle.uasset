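; GM_GlooBattle is the game mode for a Gloo battle, switching from a timed opening phase to a boss battle.
; On begin play it starts music, creates the gameplay widget and binds the player ball's death to the game-over dispatcher.
; Tick runs a slowed countdown that, on expiry, changes battle mode, swaps the music track and broadcasts the boss battle.
; It also refreshes music volume from game-instance options every tick.
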(event `self.ReceiveBeginPlay`
  (bind _returnvalue (`GameplayStatics.GetActorOfClass` "/Game/Characters/Player/BP_PlayerBall.BP_PlayerBall_C"))
  (add `/Game/Characters/Player/BP_Glooball.OnDeath` _returnvalue (delegate `GameOver`))
  (set `self.BattleTimer` 90.0)
  (bind _returnvalue_2 (`GameplayStatics.SpawnSound2D` (`|GetArrayItem` (`self.MusicTrack`)) (`/Game/Other/OptionSaveGame.GetMusicVol` (`/Game/Other/GI_GlooGameInstance.GetOptions` (`/Game/Other/GameInstance/GlooInstanceHelper.Get Gloo Game Instance`)) true) 1.0 0.0 null))
  (set `self.PlayingMusic` _returnvalue_2)
  (bind _returnvalue_3 (`|CreateWidget` "/Game/UI/Gameplay/WB_Gameplay.WB_Gameplay_C" (`GameplayStatics.GetPlayerController` 0)))
  (`UserWidget.AddToViewport` _returnvalue_3 0))

(event `GameOver`
  (`self.OnGameOver`))

(event `self.ReceiveTick`
  (params (DeltaSeconds :type "Float (single-precision)"))
  (`self.TickBattleTimer` DeltaSeconds)
  (`self.UpdateMusicVolume`))

(fn `StopMusic`
  (if (`KismetSystemLibrary.IsValid` (`self.PlayingMusic`))
    (`AudioComponent.Stop` (`self.PlayingMusic`)))
  (return))

(fn `TickBattleTimer`
  (params (DeltaTime :type "Float (double-precision)" :default 0.01))
  (if (> (`self.BattleTimer`) 0.0)
    (set `self.BattleTimer` (- (`self.BattleTimer`) (/ DeltaTime 1.3)))
    (if (<= (`self.BattleTimer`) 0.0)
      (set `self.BattleMode` "NewEnumerator1")
      (`self.StopMusic`)
      (bind _returnvalue (`GameplayStatics.SpawnSound2D` (`|GetArrayItem` (`self.MusicTrack`) 1) 1.0 1.0 0.0 null))
      (set `self.PlayingMusic` _returnvalue)
      (`self.OnBossBattle`))))

(fn `UpdateMusicVolume`
  (if (`KismetSystemLibrary.IsValid` (`self.PlayingMusic`))
    (`AudioComponent.SetVolumeMultiplier` (`self.PlayingMusic`) (`/Game/Other/OptionSaveGame.GetMusicVol` (`/Game/Other/GI_GlooGameInstance.GetOptions` (`/Game/Other/GameInstance/GlooInstanceHelper.Get Gloo Game Instance`)) true))
    (return)))

(fn `UserConstructionScript`)